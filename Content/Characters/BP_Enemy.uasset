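; BP_Enemy is an enemy NPC that takes damage and is destroyed when its health runs out.
; AnyDamage subtracts the damage from Health and prints the hit and remaining health against a hard-coded 100 HP maximum.
; At zero or below, it prints a death message and destroys the actor immediately.
; BeginPlay, overlap, Tick and the construction script are empty.
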(event `self.ReceiveAnyDamage`
  (params (Damage :type "Float (single-precision)") (DamageType :type "DamageType Object Reference") (InstigatedBy :type "Controller Object Reference") (DamageCauser :type "Actor Object Reference"))
  ; Gets Shot
  (bind _output_get (set `self.Health` (- (`self.Health`) Damage)))
  ; Log Health
  (`KismetSystemLibrary.PrintText` (`KismetTextLibrary.Conv_StringToText` (`KismetStringLibrary.Concat_StrStr` "Took damage (" (`KismetStringLibrary.Conv_DoubleToString` Damage) ") : " (`KismetStringLibrary.Conv_DoubleToString` _output_get) " / 100 HP")))
  ; Is dead?
  (if (<= _output_get 0.0)
    (`KismetSystemLibrary.PrintText` "NPC dies")
    (`self.K2_DestroyActor`)))

(fn `UserConstructionScript`)